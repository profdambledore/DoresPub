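; BP_ObjectSnapping is an actor that displays a selected static mesh and manages a list of snap points for it, apparently for editor snap setup.
; Each point is a spawned BP_SnapComponent actor given a random arrow color and selected when added.
; Functions step the selected index forward or back, remove the last point while keeping at least one, or destroy all points and force garbage collection.
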(event Custom|SetTargetMesh
  (params (StaticMesh :type Static%20Mesh%20Object%20Reference))
  (Components|StaticMesh|SetStaticMesh (Variables|Default|GetSelectedMesh) StaticMesh))

(fn ConstructionScript)

(fn AddNewSnapComponent
  (bind _returnvalue (Game|SpawnActorfromClass "/Game/Core/Editor/ObjectSnapping/BP_SnapComponent.BP_SnapComponent_C" (Transformation|GetActorTransform) "Undefined" "MultiplyWithRoot" 0 0))
  (bind _output_get (LocalVariables|SetNewSnapLoc _returnvalue))
  (Variables|/Script/Engine.ArrowComponent|SetArrowColor (Variables|/Game/Core/Editor/ObjectSnapping/BP_SnapComponent.BP_SnapComponent_C|GetSnapTransform _output_get) (Math|Conversions|ToColor(LinearColor) (Utilities|Struct|MakeLinearColor (Math|Random|RandomFloatinRange 0.0 1.0) (Math|Random|RandomFloatinRange 0.0 1.0) (Math|Random|RandomFloatinRange 0.0 1.0) 1.0)))
  (bind _returnvalue_2 (Utilities|Array|Add (Variables|Default|GetSnapLocations) (LocalVariables|GetNewSnapLoc)))
  (Variables|Default|SetSelectedIndex _returnvalue_2)
  (return (LocalVariables|GetNewSnapLoc) _returnvalue_2))

(fn RemoveSnapComponent
  (bind _snaplocations (Variables|Default|GetSnapLocations))
  (bind _returnvalue (Utilities|Array|Length _snaplocations))
  (bind _returnvalue_2 (- _returnvalue 1))
  (if (> _returnvalue_2 0)
    (bind _output_get (LocalVariables|SetActorToRemove (Utilities|Array|Get(acopy) _snaplocations _returnvalue_2)))
    (Utilities|Array|RemoveIndex _snaplocations _returnvalue_2)
    (Actor|DestroyActor _output_get)
    (Utilities|Platform|CollectGarbage)
    (if (> (Variables|Default|GetSelectedIndex) _returnvalue_2)
      (Variables|Default|SetSelectedIndex _returnvalue_2))
    (return true (Utilities|Array|Get(acopy) (Variables|Default|GetSnapLocations) _returnvalue_2) (Variables|Default|GetSelectedIndex))
    (else
      (return false 0 0))))

(fn GetNextSnapPoint
  (if (< (+ (Variables|Default|GetSelectedIndex) 1) (Utilities|Array|Length (Variables|Default|GetSnapLocations)))
    (bind _output_get (Variables|Default|SetSelectedIndex (+ (Variables|Default|GetSelectedIndex) 1)))
    (Development|PrintString (Utilities|String|ToString(Integer) (Variables|Default|GetSelectedIndex))))
  (return (Variables|Default|GetSelectedIndex) (Utilities|Array|Get(acopy) (Variables|Default|GetSnapLocations) _output_get)))

(fn GetPrevSnapPoint
  (if (>= (- (Variables|Default|GetSelectedIndex) 1) 0)
    (bind _output_get (Variables|Default|SetSelectedIndex (- (Variables|Default|GetSelectedIndex) 1))))
  (Development|PrintString (Utilities|String|ToString(Integer) (Variables|Default|GetSelectedIndex)))
  (return (Variables|Default|GetSelectedIndex) (Utilities|Array|Get(acopy) (Variables|Default|GetSnapLocations) _output_get)))

(fn DestroyAllSnapComponents
  (for _array_element (Variables|Default|GetSnapLocations)
    (Actor|DestroyActor _array_element))
  (Utilities|Array|Clear (Variables|Default|GetSnapLocations))
  (Utilities|Platform|CollectGarbage))