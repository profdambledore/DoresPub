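; BP_IconTool is an editor icon-tool actor that frames a single static mesh for a scene capture, likely to render icons.
; The construction script restricts the SceneCaptureComponent2D to show only the TargetMesh, isolating it from the rest of the scene.
; Events swap the mesh, yaw it by a scaled amount, and zoom by changing the spring arm length.
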(event Custom|ModifyRotation
  (params (RotationAmount :type Float%20%28double-precision%29) (Multi :type Integer))
  (Transformation|AddLocalRotation (Variables|Default|GetTargetMesh) (Math|Rotator|MakeRotator 0.0 0.0 (* RotationAmount Multi)) false false)
  (Development|PrintString "Updating Rotation"))

(event Custom|ModifyZoom
  (params (ZoomAmount :type Float%20%28double-precision%29) (Multi :type Integer))
  (bind _springarm (Variables|Default|GetSpringArm))
  (Variables|/Script/Engine.SpringArmComponent|SetTargetArmLength _springarm (+ (Variables|/Script/Engine.SpringArmComponent|GetTargetArmLength _springarm) (* ZoomAmount Multi))))

(event Custom|SetTargetMesh
  (params (StaticMesh :type Static%20Mesh%20Object%20Reference))
  (Components|StaticMesh|SetStaticMesh (Variables|Default|GetTargetMesh) StaticMesh))

(fn ConstructionScript
  (Rendering|SceneCapture|ShowOnlyComponent (Variables|Default|GetSceneCaptureComponent2D) (Variables|Default|GetTargetMesh))
  (Development|PrintString "Hello"))