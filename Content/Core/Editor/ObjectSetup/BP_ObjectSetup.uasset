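; BP_ObjectSetup is an editor preview actor for setting up snap points on a static mesh.
; A SceneCapture2D renders only the target mesh, while events rotate, zoom and pan the spring arm.
; Functions spawn randomly colored BP_SnapComponent actors with snap type, snap-with and hover offset settings, remove the last or all of them, and step a clamped selection index through the list.
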(event Custom|ModifyRotation
  (params (RotationAmount :type Float%20%28double-precision%29) (Multi :type Integer))
  (Transformation|AddLocalRotation (Variables|Default|GetSpringArm) (Math|Rotator|MakeRotator 0.0 0.0 (* RotationAmount Multi)) false false))

(event Custom|ModifyZoom
  (params (ZoomAmount :type Float%20%28double-precision%29) (Multi :type Integer))
  (bind _springarm (Variables|Default|GetSpringArm))
  (Variables|/Script/Engine.SpringArmComponent|SetTargetArmLength _springarm (+ (Variables|/Script/Engine.SpringArmComponent|GetTargetArmLength _springarm) (* ZoomAmount Multi))))

(event Custom|SetTargetMesh
  (params (StaticMesh :type Static%20Mesh%20Object%20Reference))
  (Components|StaticMesh|SetStaticMesh (Variables|Default|GetTargetMesh) StaticMesh))

(event Custom|ModZ
  (params (MovementAmount :type Float%20%28double-precision%29) (Multi :type Integer))
  (Transformation|AddWorldOffset (Variables|Default|GetSpringArm) (Math|Vector|MakeVector 0.0 0.0 (* MovementAmount Multi)) false false))

(event Custom|ModifyX
  (params (MovementAmount :type Float%20%28double-precision%29) (Multi :type Integer))
  (bind _springarm (Variables|Default|GetSpringArm))
  (Transformation|AddWorldOffset _springarm (* (Math|Vector|GetRightVector _springarm) (* MovementAmount Multi)) false false))

(fn ConstructionScript
  (Rendering|SceneCapture|ShowOnlyComponent (Variables|Default|GetSceneCaptureComponent2D) (Variables|Default|GetTargetMesh)))

(fn AddSnapPoint
  (params (SnapTransform :type Transform) (OffsetLocation :type Vector) (SnapType :type Name) (SnapWith :type Name))
  (bind _returnvalue (Transformation|GetActorTransform))
  (bind _returnvalue_2 (Game|SpawnActorfromClass "/Game/Core/Editor/ObjectSnapping/BP_SnapComponent.BP_SnapComponent_C" (Math|Transform|MakeTransform (+ (.location SnapTransform) (.location _returnvalue)) (.rotation SnapTransform) (.scale _returnvalue)) "Undefined" "MultiplyWithRoot" 0 0))
  (bind _output_get (LocalVariables|SetNewSnapLoc _returnvalue_2))
  (Transformation|SetRelativeLocation (Variables|/Game/Core/Editor/ObjectSnapping/BP_SnapComponent.BP_SnapComponent_C|GetHoverOffset _returnvalue_2) OffsetLocation false false)
  (Variables|/Script/Engine.ArrowComponent|SetArrowColor (Variables|/Game/Core/Editor/ObjectSnapping/BP_SnapComponent.BP_SnapComponent_C|GetSnapTransform _output_get) (Math|Conversions|ToColor(LinearColor) (Utilities|Struct|MakeLinearColor (Math|Random|RandomFloatinRange 0.0 1.0) (Math|Random|RandomFloatinRange 0.0 1.0) (Math|Random|RandomFloatinRange 0.0 1.0) 1.0)))
  (bind _returnvalue_3 (Utilities|Array|Add (Variables|Default|GetSnapLocations) (LocalVariables|GetNewSnapLoc)))
  (Variables|Default|SetSelectedIndex _returnvalue_3)
  (Default|SetSnapType (LocalVariables|GetNewSnapLoc) SnapType)
  (Default|SetSnapwith (LocalVariables|GetNewSnapLoc) SnapWith)
  (return (LocalVariables|GetNewSnapLoc) _returnvalue_3))

(fn RemoveSnapPoint
  (bind _snaplocations (Variables|Default|GetSnapLocations))
  (bind _returnvalue (Utilities|Array|Length _snaplocations))
  (bind _returnvalue_2 (- _returnvalue 1))
  (if (Utilities|Array|IsEmpty _snaplocations)
    (return false 0 0)
    (else
      (LocalVariables|SetActorToRemvoe (Utilities|Array|Get(acopy) _snaplocations _returnvalue_2))
      (Utilities|Array|RemoveIndex _snaplocations _returnvalue_2)
      (Actor|DestroyActor (LocalVariables|GetActorToRemvoe))
      (Utilities|Platform|CollectGarbage)
      (if (Utilities|Array|IsEmpty (Variables|Default|GetSnapLocations))
        (bind _output_get (Variables|Default|SetSelectedIndex -1))
        (return true 0 _output_get)
        (else
          (if (> (Variables|Default|GetSelectedIndex) _returnvalue_2)
            (Variables|Default|SetSelectedIndex _returnvalue_2))
          (return true (Utilities|Array|Get(acopy) (Variables|Default|GetSnapLocations)) (Variables|Default|GetSelectedIndex)))))))

(fn DestroyAllSnapPoints
  (for _array_element (Variables|Default|GetSnapLocations)
    (Actor|DestroyActor _array_element))
  (Utilities|Array|Clear (Variables|Default|GetSnapLocations))
  (Utilities|Platform|CollectGarbage))

(fn GetNextSnapPoint
  (bind _snaplocations (Variables|Default|GetSnapLocations))
  (if (Utilities|Array|IsEmpty _snaplocations)
    (return 0 0 false)
    (else
      (if (< (+ (Variables|Default|GetSelectedIndex) 1) (Utilities|Array|Length _snaplocations))
        (bind _output_get (Variables|Default|SetSelectedIndex (+ (Variables|Default|GetSelectedIndex) 1))))
      (return (Variables|Default|GetSelectedIndex) (Utilities|Array|Get(acopy) (Variables|Default|GetSnapLocations) _output_get) true))))

(fn GetPrevSnapPoint
  (if (Utilities|Array|IsEmpty (Variables|Default|GetSnapLocations))
    (return 0 0 false)
    (else
      (if (>= (- (Variables|Default|GetSelectedIndex) 1) 0)
        (bind _output_get (Variables|Default|SetSelectedIndex (- (Variables|Default|GetSelectedIndex) 1))))
      (Development|PrintString (Utilities|String|ToString(Integer) (Variables|Default|GetSelectedIndex)))
      (return (Variables|Default|GetSelectedIndex) (Utilities|Array|Get(acopy) (Variables|Default|GetSnapLocations) _output_get) true))))